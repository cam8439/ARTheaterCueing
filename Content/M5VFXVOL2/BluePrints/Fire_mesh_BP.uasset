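; Fire mesh Blueprint that pairs a configurable static mesh with a fire particle effect.
; The construction script applies mesh and scale, and BeginPlay sets the particle template, offset, scale and optional smoke and distortion emitters.
; Tick copies mesh movement into a Transform variable, whose OnRep moves the mesh.
; ClientSetVisibility sets Visible, whose OnRep toggles the particles, while ClientSetTransform is an empty stub.
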(event `self.ReceiveBeginPlay`
  (bind _particlesystem (`self.Particlesystem`))
  (set `self.Transform` (`SceneComponent.K2_GetComponentToWorld` (`self.StaticMeshComponent`)))
  (`ParticleSystemComponent.SetTemplate` _particlesystem (`self.particle_fire`))
  (`SceneComponent.K2_SetRelativeLocation` _particlesystem (`self.Particle_offset`) false false)
  (`SceneComponent.SetRelativeScale3D` _particlesystem (`self.Particle_Scale`))
  (`ParticleSystemComponent.SetEmitterEnable` (`self.ParticleSystem`) "smoke" (`self.Smoke_Emitter_Enable`))
  (`ParticleSystemComponent.SetEmitterEnable` (`self.ParticleSystem`) "Distortion" (`self.Distortion_Emittter_Enable`)))

(event `self.ReceiveTick`
  (params (DeltaSeconds :type "Float (single-precision)"))
  (bind _returnvalue (`SceneComponent.K2_GetComponentToWorld` (`self.StaticMeshComponent`)))
  (if (not (== (`self.Transform`) _returnvalue))
    (set `self.Transform` _returnvalue)))

(event `Client Set Visibility`
  (params (client_visible :type Boolean))
  (set `self.Visible` client_visible))

(event `Client Set Transform`
  (params (`new transform` :type "Transform Structure")))

(fn `OnRep_Transform`
  (`SceneComponent.K2_SetWorldTransform` (`self.StaticMeshComponent`) (`self.Transform`) false false))

(fn `OnRep_Visible`
  (`SceneComponent.SetVisibility` (`self.Particlesystem`) (`self.Visible`) true))

(fn `UserConstructionScript`
  (bind _staticmeshcomponent (`self.StaticMeshComponent`))
  (`StaticMeshComponent.SetStaticMesh` _staticmeshcomponent (`self.Staticmesh`))
  (`SceneComponent.SetRelativeScale3D` _staticmeshcomponent (`self.Scale`)))