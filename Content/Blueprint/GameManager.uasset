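; GameManager Blueprint that spawns a single DragonMarker once an origin image has been found.
; Each Tick it polls CoordinateSyncRef until the origin is found, using a flag to ensure the spawn happens only once.
; The marker is placed at a downward offset from the origin image's location and takes that image's rotation combined with a half-turn offset.
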(event `self.ReceiveTick`
  (params (DeltaSeconds :type "Float (single-precision)"))
  (bind _coordinatesyncref (`self.CoordinateSyncRef`))
  (if (and (`/Game/Blueprint/CoordinateSync.OriginFound` _coordinatesyncref) (not (`self.Dragonspawned`)))
    (bind _returnvalue (`|SpawnActorFromClass` "/Game/Blueprint/DragonMarker.DragonMarker_C" (`KismetMathLibrary.Conv_VectorToTransform` (+ (`/Game/Blueprint/CoordinateSync.OriginImageLocation` _coordinatesyncref) (0.0 0.0 -80.0))) "Undefined" "OverrideRootScale" null null))
    (`self.K2_SetActorRotation` _returnvalue (`KismetMathLibrary.ComposeRotators` (`/Game/Blueprint/CoordinateSync.OriginImageRotation` _coordinatesyncref) (struct :`Yaw` 180.0)) false)
    (set `self.Dragonspawned` true)))

(fn `UserConstructionScript`)