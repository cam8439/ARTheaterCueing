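; BP_ImageTracker is a Magic Leap image-tracking actor that spawns a DragonMarker and anchors it to a detected image target.
; When the target is found it sets a detection flag; on Tick it spawns the dragon once at the hidden Cube, then keeps matching Cube location and tracker rotation at reduced scale.
; A text render shows the tracker's world location.
; Losing the target does not clear the flag, so updates continue.
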(event `self.ReceiveBeginPlay`
  (bind _magicleapimagetracker (`self.MagicLeapImageTracker`))
  (`SceneComponent.SetHiddenInGame` (`self.Cube`) true true)
  (`self.K2_SetActorLocation` (`SceneComponent.K2_GetComponentLocation` _magicleapimagetracker) true)
  (`self.K2_SetActorRotation` (`SceneComponent.K2_GetComponentRotation` _magicleapimagetracker)))

(event `self.ReceiveTick`
  (params (DeltaSeconds :type "Float (single-precision)"))
  (bind _characterref (`self.CharacterRef`))
  (bind _magicleapimagetracker (`self.MagicLeapImageTracker`))
  (bind _returnvalue (`SceneComponent.K2_GetComponentLocation` (`self.Cube`)))
  (bind _returnvalue_2 (`SceneComponent.K2_GetComponentRotation` _magicleapimagetracker))
  (`TextRenderComponent.K2_SetText` (`self.TextRender`) (`KismetTextLibrary.Conv_VectorToText` (`SceneComponent.K2_GetComponentLocation` _magicleapimagetracker)))
  (if (`self.Character_spawned`)
    (if (`self.Image_detected`)
      (`self.K2_SetActorLocation` _characterref _returnvalue false false)
      (`self.K2_SetActorRotation` _characterref _returnvalue_2 false)
      (`self.SetActorScale3D` _characterref (0.1 0.1 0.1)))
    (elif (`self.Image_detected`)
      (bind _returnvalue_3 (`|SpawnActorFromClass` "/Game/Blueprint/DragonMarker.DragonMarker_C" (`KismetMathLibrary.Conv_VectorToTransform` _returnvalue) "Undefined" "OverrideRootScale" null null))
      (bind _output_get (set `self.CharacterRef` _returnvalue_3))
      (`self.K2_SetActorRotation` _output_get _returnvalue_2 false)
      (set `self.Character_spawned` true))))

(event `self.MagicLeapImageTracker.OnImageTargetFound`
  (`SceneComponent.SetHiddenInGame` (`self.Cube`) true true)
  (set `self.Image_detected` true))

(event `self.MagicLeapImageTracker.OnImageTargetLost`
  (`SceneComponent.SetHiddenInGame` (`self.Cube`) true true))

(fn `UserConstructionScript`)