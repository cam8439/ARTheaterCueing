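; Magic Leap actor that turns a tracked image target into a world origin for placing a referenced coordinate actor.
; Each tick it accumulates tracking time, reset on target loss, and latches the tracker's location and rotation after three seconds.
; It then moves and reveals that actor once, lowered from the saved location; saved rotation stays unapplied.
; Timer and location debug texts update every tick but start hidden.
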(event `self.ReceiveBeginPlay`
  (`SceneComponent.SetHiddenInGame` (`self.Cube`) true false)
  (`SceneComponent.SetHiddenInGame` (`self.Timer`) true false)
  (`SceneComponent.SetHiddenInGame` (`self.Origin_Text`) true false)
  (`SceneComponent.SetHiddenInGame` (`self.Debug_text`) true false))

(event `self.ReceiveTick`
  (params (DeltaSeconds :type "Float (single-precision)"))
  (`self.RecordTrackingTime` DeltaSeconds)
  (`self.DisplayTrackingTime`)
  (`self.SetImageOrigins`)
  (`self.DisplayOrigins`)
  (`self.SetImageCoordinate`))

(event `self.MagicLeapImageTracker.OnImageTargetFound`
  (set `self.ImageFound` true))

(event `self.MagicLeapImageTracker.OnImageTargetLost`
  (set `self.ImageFound` false)
  (set `self.TrackedTime` 0.0))

(fn `DisplayOrigins`
  (`TextRenderComponent.K2_SetText` (`self.Origin_Text`) (`KismetTextLibrary.Conv_VectorToText` (`SceneComponent.K2_GetComponentLocation` (`self.MagicLeapImageTracker`))))
  (`TextRenderComponent.K2_SetText` (`self.Debug_text`) (`KismetTextLibrary.Conv_VectorToText` (`SceneComponent.K2_GetComponentLocation` (`self.Cube`)))))

(fn `DisplayTrackingTime`
  (if (`self.OriginFound`)
    (`TextRenderComponent.K2_SetText` (`self.Timer`) (`self.Origin Found Indicator`))
    (else
      (`TextRenderComponent.K2_SetText` (`self.Timer`) (`KismetTextLibrary.Conv_DoubleToText` (`self.TrackedTime`) "HalfToEven")))))

(fn `RecordTrackingTime`
  (params (`delta time` :type "Float (double-precision)"))
  (if (and (`self.ImageFound`) (not (`self.OriginFound`)))
    (set `self.TrackedTime` (+ `delta time` (`self.TrackedTime`)))))

(fn `SetImageCoordinate`
  (if (and (not (`self.CoordSet`)) (`self.OriginFound`))
    (`self.K2_SetActorLocation` (`self.ImageCoordRef`) (+ (`self.OriginImageLocation`) (0.0 0.0 -100.0)) false false)
    (`self.SetActorHiddenInGame` (`self.ImageCoordRef`) false)
    (set `self.CoordSet` true)))

(fn `SetImageOrigins`
  (bind _magicleapimagetracker (`self.MagicLeapImageTracker`))
  (if (and (>= (`self.TrackedTime`) 3.0) (not (`self.OriginFound`)))
    (set `self.OriginImageLocation` (`SceneComponent.K2_GetComponentLocation` _magicleapimagetracker))
    (set `self.OriginImageRotation` (`SceneComponent.K2_GetComponentRotation` _magicleapimagetracker))
    (set `self.OriginFound` true)))

(fn `UserConstructionScript`)