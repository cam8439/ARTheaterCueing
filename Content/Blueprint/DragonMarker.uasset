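; DragonMarker is a debug-style marker actor that displays its position relative to an origin image tracked by the game manager's CoordinateSync reference.
; Every Tick, it subtracts OriginImageLocation from its root's world location and writes the result to RelativeLocationIndicator.
; RelativeRotationIndicator shows the world location minus the X vector of OriginImageRotation, so it holds a vector difference rather than a relative rotation.
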(event `self.ReceiveTick`
  (params (DeltaSeconds :type "Float (single-precision)"))
  (`TextRenderComponent.K2_SetText` (`self.RelativeLocationIndicator`) (`KismetTextLibrary.Conv_VectorToText` (- (`SceneComponent.K2_GetComponentLocation` (`self.DefaultSceneRoot`)) (`/Game/Blueprint/CoordinateSync.OriginImageLocation` (`/Game/Blueprint/GameManager.CoordinateSyncRef` (`self.GameManagerRef`))))))
  (`TextRenderComponent.K2_SetText` (`self.RelativeRotationIndicator`) (`KismetTextLibrary.Conv_VectorToText` (- (`SceneComponent.K2_GetComponentLocation` (`self.DefaultSceneRoot`)) (`KismetMathLibrary.Conv_RotatorToVector` (`/Game/Blueprint/CoordinateSync.OriginImageRotation` (`/Game/Blueprint/GameManager.CoordinateSyncRef` (`self.GameManagerRef`))))))))

(fn `UserConstructionScript`)