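; CueManager is a replicated actor that creates cues in an external OSC cue app (QLab-style addresses) from the level's sequences.
; GetAllSequences finds every LevelSequenceActor, tags it with its object name, and sends a prefixed "new osc" message through the supplied OSC client.
; It then builds custom-string (actor name) and patch messages for the selected cue, using OSC bundles to send settings.
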(fn `Get All Sequences`
  (params (OSCClient :type "OSCClient Object Reference") (Prefix :type String))
  (locals (name :type String))
  (bind _oscbundle (make `OSCBundle`))
  (bind _outactors (`GameplayStatics.GetAllActorsOfClass` "/Script/LevelSequence.LevelSequenceActor"))
  (for _array_element _outactors
    (bind _returnvalue (`KismetSystemLibrary.GetObjectName` _array_element))
    (`KismetArrayLibrary.Array_Insert` (`Actor.Tags` _array_element) (`KismetStringLibrary.Conv_StringToName` _returnvalue))
    (bind _returnvalue_2 (`OSCManager.ConvertStringToOSCAddress` (`KismetStringLibrary.Concat_StrStr` Prefix "/new osc")))
    (bind _returnvalue_3 (`OSCManager.SetOSCMessageAddress` (make `OSCMessage`) _returnvalue_2))
    (`OSCClient.SendOSCMessage` OSCClient _returnvalue_3)
    (bind _returnvalue_4 (`OSCManager.ConvertStringToOSCAddress` "/cue/selected/customString"))
    (bind _returnvalue_5 (`OSCManager.SetOSCMessageAddress` (make `OSCMessage`) _returnvalue_4))
    (bind _output_get (set `local.name` _returnvalue))
    (bind _returnvalue_6 (`OSCManager.AddString` _returnvalue_5 _output_get))
    (bind _returnvalue_7 (`OSCManager.ConvertStringToOSCAddress` "/cue/selected/patch"))
    (bind _returnvalue_8 (`OSCManager.SetOSCMessageAddress` (make `OSCMessage`) _returnvalue_7))
    (bind _returnvalue_9 (`OSCManager.AddInt32` _returnvalue_8 2))
    (`OSCManager.AddMessageToBundle` _returnvalue_6 _oscbundle)
    (bind _returnvalue_10 (`OSCManager.AddMessageToBundle` _returnvalue_9 _oscbundle))
    (`OSCClient.SendOSCBundle` OSCClient _returnvalue_10)))

(fn `UserConstructionScript`
  (`self.SetReplicates` true))