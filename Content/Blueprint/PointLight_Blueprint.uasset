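; Point light Blueprint that keeps its light color in sync over the network through a replicated CurrentColor variable.
; BeginPlay sets CurrentColor to white, and Tick polls the light component's color, copying it into the variable whenever it differs.
; The RepNotify applies CurrentColor to the point light component as an sRGB color.
; Neither BeginPlay nor Tick checks for network authority.
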(event `self.ReceiveBeginPlay`
  (set `self.current color` (make `LinearColor` 1.0 1.0 1.0)))

(event `self.ReceiveTick`
  (params (DeltaSeconds :type "Float (single-precision)"))
  (bind _returnvalue (`LightComponentBase.GetLightColor` (`self.LightComponent`)))
  (if (not (== (`self.current color`) _returnvalue))
    (set `self.current color` _returnvalue)))

(fn `OnRep_current color`
  (`LightComponent.SetLightColor` (`self.PointLightComponent`) (`self.current color`) true))

(fn `UserConstructionScript`)